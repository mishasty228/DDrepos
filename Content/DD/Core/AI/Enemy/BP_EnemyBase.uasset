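; BP_EnemyBase is an enemy base Blueprint with health, a melee punch and a spawned weapon.
; On BeginPlay it links itself to its UI_Health widget, then spawns the Hand class as its weapon, attached to a scene component with itself as holder.
; MeleeAttack plays the punch montage, holding an Attack flag until it completes.
; Incoming damage lowers Health, and reaching zero triggers Death once, destroying weapon and enemy.
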(event Custom|getDamage
  (params (Damage :type Integer))
  (bind _output_get (Variables|Default|SetHealth (- (Variables|Default|GetHealth) Damage)))
  (if (<= _output_get 0)
    (Utilities|FlowControl|DoOnce false
      (:Completed
        (CallFunction|Death)))))

(event Custom|Attack
  (Variables|Default|SetAttack? true)
  (Animation|Montage|PlayMontage (Variables|Character|GetMesh) "/Game/DD/Core/Animations/Punch_Anim.Punch_Anim"
    (:OnCompleted
      (Variables|Default|SetAttack? false)
      (Development|PrintString "Punch"))))

(event Custom|Death
  (Actor|DestroyActor (Variables|Default|GetWeapon))
  (Actor|DestroyActor))

(event EventBeginPlay
  (bind _scene (Variables|Default|GetScene))
  (bind _asui_health (Utilities|Casting|CastToUI_Health (UserInterface|GetUserWidgetObject (Variables|Default|GetWidget))))
  (Variables|/Game/DD/Core/AI/UI_Health.UI_Health_C|SetEnemy _asui_health self)
  (bind _returnvalue (Game|SpawnActorfromClass "/Game/DD/Core/Inventory/Weapons/hand.hand_C" (Math|Transform|MakeTransform (Transformation|GetWorldLocation _scene) "0, 0, 0" "1,1,1") "Undefined" 0 0))
  (Variables|Default|SetWeapon _returnvalue)
  (Transformation|AttachComponentToComponent _returnvalue _scene "None" "SnapToTarget" "SnapToTarget" "SnapToTarget" true)
  (Variables|/Game/DD/Core/Inventory/Weapons/hand.hand_C|SetHolder _returnvalue self))

(event EventMeleeAttack
  (CallFunction|Attack))

(fn ConstructionScript)
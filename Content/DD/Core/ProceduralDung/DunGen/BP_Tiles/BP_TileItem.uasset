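; BP_TileItem is a procedural dungeon tile that spawns one random loot actor on itself when play begins.
; BeginPlay calls the parent tile logic, then picks a point randomly offset in X and Y around the Floor1 component and slightly above it.
; A uniform random switch spawns one of six potion classes or a chest container, with only the chest getting a random yaw.
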(event EventBeginPlay
  (bind _floor1 (Variables|Default|Getfloor1))
  (bind _returnvalue (Transformation|GetWorldLocation _floor1))
  (|CallParentFunction)
  (Variables|Default|SetSpawnLoc (Math|Vector|MakeVector (Math|Random|RandomFloatinRange (- (.x _returnvalue) 1e+02) (+ (.x _returnvalue) 1e+02)) (Math|Random|RandomFloatinRange (- (.y _returnvalue) 1e+02) (+ (.y _returnvalue) 1e+02)) (+ (.z _returnvalue) 1e+01)))
  (bind _output_get (Variables|Default|SetSpawn%20value (Math|Random|RandomIntegerinRange 0 6)))
  (switch int _output_get
    (:0
      (Game|SpawnActorfromClass "/Game/DD/Core/Inventory/Items/Potion_1.Potion_1_C" (Math|Transform|MakeTransform (Variables|Default|GetSpawnLoc) "0, 0, 0" "1,1,1") "Undefined" 0 0))
    (:1
      (Game|SpawnActorfromClass "/Game/DD/Core/Inventory/Items/Potion_2.Potion_2_C" (Math|Transform|MakeTransform (Variables|Default|GetSpawnLoc) "0, 0, 0" "1,1,1") "Undefined" 0 0))
    (:2
      (Game|SpawnActorfromClass "/Game/DD/Core/Inventory/Items/Potion_3.Potion_3_C" (Math|Transform|MakeTransform (Variables|Default|GetSpawnLoc) "0, 0, 0" "1,1,1") "Undefined" 0 0))
    (:3
      (Game|SpawnActorfromClass "/Game/DD/Core/Inventory/Items/Potion_4.Potion_4_C" (Math|Transform|MakeTransform (Variables|Default|GetSpawnLoc) "0, 0, 0" "1,1,1") "Undefined" 0 0))
    (:4
      (Game|SpawnActorfromClass "/Game/DD/Core/Inventory/Items/Potion_5.Potion_5_C" (Math|Transform|MakeTransform (Variables|Default|GetSpawnLoc) "0, 0, 0" "1,1,1") "Undefined" 0 0))
    (:5
      (Game|SpawnActorfromClass "/Game/DD/Core/Inventory/Items/Potion_6.Potion_6_C" (Math|Transform|MakeTransform (Variables|Default|GetSpawnLoc) "0, 0, 0" "1,1,1") "Undefined" 0 0))
    (:6
      (Game|SpawnActorfromClass "/Game/DD/Core/Inventory/ChestContainer.ChestContainer_C" (Math|Transform|MakeTransform (Variables|Default|GetSpawnLoc) (Math|Rotator|MakeRotator 0.0 0.0 (Math|Random|RandomFloatinRange 0.0 3.6e+02)) "1,1,1") "Undefined" 0 0))))

(fn ConstructionScript
  (|CallParentFunction))
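; BP_DoorTile is a procedural dungeon tile that populates itself with doors.
; On BeginPlay it spawns a BP_ArcDoor at the world transform of each of its four Scene components.
; When BP_Player begins overlapping Box_0, the tile's Plane switches to the Yellow material, with no logic to revert it.
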(event OnComponentBeginOverlap(Box_0)
  (params (OverlappedComponent :type Primitive%20Component%20Object%20Reference) (OtherActor :type Actor%20Object%20Reference) (OtherComp :type Primitive%20Component%20Object%20Reference) (OtherBodyIndex :type Integer) (bFromSweep :type Boolean) (SweepResult :type Hit%20Result%20Structure%20%28by%20ref%29))
  (Utilities|Casting|CastToBP_Player OtherActor)
  (Rendering|Material|SetMaterial (Variables|Default|GetPlane) 0 "/Game/DD/Models/Dung/Yellow.Yellow"))

(event EventBeginPlay
  (Game|SpawnActorfromClass "/Game/DD/Core/ProceduralDung/BP_Tiles/parts/BP_ArcDoor.BP_ArcDoor_C" (Transformation|GetWorldTransform (Variables|Default|GetScene)) "Undefined" 0 0)
  (Game|SpawnActorfromClass "/Game/DD/Core/ProceduralDung/BP_Tiles/parts/BP_ArcDoor.BP_ArcDoor_C" (Transformation|GetWorldTransform (Variables|Default|GetScene1)) "Undefined" 0 0)
  (Game|SpawnActorfromClass "/Game/DD/Core/ProceduralDung/BP_Tiles/parts/BP_ArcDoor.BP_ArcDoor_C" (Transformation|GetWorldTransform (Variables|Default|GetScene2)) "Undefined" 0 0)
  (Game|SpawnActorfromClass "/Game/DD/Core/ProceduralDung/BP_Tiles/parts/BP_ArcDoor.BP_ArcDoor_C" (Transformation|GetWorldTransform (Variables|Default|GetScene3)) "Undefined" 0 0))

(fn ConstructionScript)
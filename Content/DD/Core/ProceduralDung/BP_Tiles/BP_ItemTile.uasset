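; Procedural dungeon item tile that spawns a random pickup when play begins.
; A uniform random roll picks one of six potion classes or a chest container, placed at the Scene component's location, with the chest given a random yaw.
; When BP_Player overlaps the tile's box, the Plane's material switches to Band.
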(event OnComponentBeginOverlap(Box_0)
  (params (OverlappedComponent :type Primitive%20Component%20Object%20Reference) (OtherActor :type Actor%20Object%20Reference) (OtherComp :type Primitive%20Component%20Object%20Reference) (OtherBodyIndex :type Integer) (bFromSweep :type Boolean) (SweepResult :type Hit%20Result%20Structure%20%28by%20ref%29))
  (Utilities|Casting|CastToBP_Player OtherActor)
  (Rendering|Material|SetMaterial (Variables|Default|GetPlane) 0 "/Game/RandomizedDungeons/chars/Band.Band"))

(event EventBeginPlay
  (Variables|Default|SetSpawnTransform (Transformation|GetWorldTransform (Variables|Default|GetScene)))
  (bind _output_get (Variables|Default|SetSpawnValue (Math|Random|RandomIntegerinRange 1 7)))
  (switch int _output_get
    (:1
      (Game|SpawnActorfromClass "/Game/DD/Core/Inventory/Items/Potion_1.Potion_1_C" (Variables|Default|GetSpawnTransform) "Undefined" 0 0))
    (:2
      (Game|SpawnActorfromClass "/Game/DD/Core/Inventory/Items/Potion_2.Potion_2_C" (Variables|Default|GetSpawnTransform) "Undefined" 0 0))
    (:3
      (Game|SpawnActorfromClass "/Game/DD/Core/Inventory/Items/Potion_3.Potion_3_C" (Variables|Default|GetSpawnTransform) "Undefined" 0 0))
    (:4
      (Game|SpawnActorfromClass "/Game/DD/Core/Inventory/Items/Potion_4.Potion_4_C" (Variables|Default|GetSpawnTransform) "Undefined" 0 0))
    (:5
      (Game|SpawnActorfromClass "/Game/DD/Core/Inventory/Items/Potion_5.Potion_5_C" (Variables|Default|GetSpawnTransform) "Undefined" 0 0))
    (:6
      (Game|SpawnActorfromClass "/Game/DD/Core/Inventory/Items/Potion_6.Potion_6_C" (Variables|Default|GetSpawnTransform) "Undefined" 0 0))
    (:7
      (bind _returnvalue (Game|SpawnActorfromClass "/Game/DD/Core/Inventory/ChestContainer.ChestContainer_C" (Math|Transform|MakeTransform (.location (Variables|Default|GetSpawnTransform)) "0, 0, 0" "1,1,1") "Undefined" 0 0))
      (Transformation|SetActorRelativeRotation _returnvalue (Math|Rotator|MakeRotator 0.0 0.0 (Math|Random|RandomFloatinRange 0.0 3.6e+02))))))

(event Collision|EventActorBeginOverlap
  (params (OtherActor :type Actor%20Object%20Reference)))

(event EventTick
  (params (DeltaSeconds :type Float%20%28single-precision%29)))

(fn ConstructionScript)
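; BP_Wall is a wall tile for the procedural dungeon that randomly decorates itself with torches.
; On BeginPlay, a single random roll gives it roughly even odds of spawning Walltorch actors at all four of its Scene component transforms, so it gets every torch or none.
; The construction script is empty, and no other events do any work.
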(event EventBeginPlay
  (if (> (Math|Random|RandomFloat) 0.5)
    (Game|SpawnActorfromClass "/Game/DD/Core/ProceduralDung/BP_Tiles/parts/walltorch.walltorch_C" (Transformation|GetWorldTransform (Variables|Default|GetScene)) "Undefined" 0 0)
    (Game|SpawnActorfromClass "/Game/DD/Core/ProceduralDung/BP_Tiles/parts/walltorch.walltorch_C" (Transformation|GetWorldTransform (Variables|Default|GetScene1)) "Undefined" 0 0)
    (Game|SpawnActorfromClass "/Game/DD/Core/ProceduralDung/BP_Tiles/parts/walltorch.walltorch_C" (Transformation|GetWorldTransform (Variables|Default|GetScene2)) "Undefined" 0 0)
    (Game|SpawnActorfromClass "/Game/DD/Core/ProceduralDung/BP_Tiles/parts/walltorch.walltorch_C" (Transformation|GetWorldTransform (Variables|Default|GetScene3)) "Undefined" 0 0)))

(event Collision|EventActorBeginOverlap
  (params (OtherActor :type Actor%20Object%20Reference)))

(event EventTick
  (params (DeltaSeconds :type Float%20%28single-precision%29)))

(fn ConstructionScript)
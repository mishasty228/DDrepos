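; BP_FallTile is a procedural dungeon tile that marks when the player has entered it.
; On BeginPlay it destroys its Head component and three extra static mesh components.
; When BP_Player begins overlapping Box_0, the Plane switches to the Blue material and is never reset here.
; Despite the name, the graphs contain no falling logic.
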(event OnComponentBeginOverlap(Box_0)
  (params (OverlappedComponent :type Primitive%20Component%20Object%20Reference) (OtherActor :type Actor%20Object%20Reference) (OtherComp :type Primitive%20Component%20Object%20Reference) (OtherBodyIndex :type Integer) (bFromSweep :type Boolean) (SweepResult :type Hit%20Result%20Structure%20%28by%20ref%29))
  (Utilities|Casting|CastToBP_Player OtherActor)
  (Rendering|Material|SetMaterial (Variables|Default|GetPlane) 0 "/Game/DD/Models/Dung/Blue.Blue"))

(event EventBeginPlay
  (Components|DestroyComponent (Variables|Default|GetHead))
  (Components|DestroyComponent (Variables|Default|GetStaticMesh2))
  (Components|DestroyComponent (Variables|Default|GetStaticMesh3))
  (Components|DestroyComponent (Variables|Default|GetStaticMesh4)))

(event Collision|EventActorBeginOverlap
  (params (OtherActor :type Actor%20Object%20Reference)))

(event EventTick
  (params (DeltaSeconds :type Float%20%28single-precision%29)))

(fn ConstructionScript)
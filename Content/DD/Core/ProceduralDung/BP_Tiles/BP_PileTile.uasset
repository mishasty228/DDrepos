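; Procedural dungeon tile that places a randomly chosen pile variant and reacts to the player entering it.
; On BeginPlay it adds an instance to one of three instanced components (Col1–Col3), using the Scene component's relative location and scale with a random yaw.
; When BP_Player overlaps the box, the Plane's material switches to Blue.
; The construction script is empty, with a disconnected world-transform version of the spawn logic left in it.
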(event OnComponentBeginOverlap(Box_0)
  (params (OverlappedComponent :type Primitive%20Component%20Object%20Reference) (OtherActor :type Actor%20Object%20Reference) (OtherComp :type Primitive%20Component%20Object%20Reference) (OtherBodyIndex :type Integer) (bFromSweep :type Boolean) (SweepResult :type Hit%20Result%20Structure%20%28by%20ref%29))
  (Utilities|Casting|CastToBP_Player OtherActor)
  (Rendering|Material|SetMaterial (Variables|Default|GetPlane) 0 "/Game/DD/Models/Dung/Blue.Blue"))

(event EventBeginPlay
  (bind _returnvalue (Math|Random|RandomFloatinRange 0.0 3.6e+02))
  (bind _scene (Variables|Default|GetScene))
  (bind _returnvalue_2 (Transformation|GetRelativeTransform _scene))
  (switch int (Math|Random|RandomIntegerinRange 0 2)
    (:0
      (Components|InstancedStaticMesh|AddInstance (Variables|Default|GetCol1) (Math|Transform|MakeTransform (.location _returnvalue_2) (Math|Rotator|MakeRotator 0.0 0.0 _returnvalue) (.scale _returnvalue_2))))
    (:1
      (Components|InstancedStaticMesh|AddInstance (Variables|Default|GetCol2) (Math|Transform|MakeTransform (.location _returnvalue_2) (Math|Rotator|MakeRotator 0.0 0.0 _returnvalue) (.scale _returnvalue_2))))
    (:2
      (Components|InstancedStaticMesh|AddInstance (Variables|Default|GetCol3) (Math|Transform|MakeTransform (.location _returnvalue_2) (Math|Rotator|MakeRotator 0.0 0.0 _returnvalue) (.scale _returnvalue_2))))))

(event Collision|EventActorBeginOverlap
  (params (OtherActor :type Actor%20Object%20Reference)))

(event EventTick
  (params (DeltaSeconds :type Float%20%28single-precision%29)))

(fn ConstructionScript)
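; Procedural dungeon tile that advances the run through streamed maps when the player overlaps its Restart volume.
; The overlap messages the current streaming level, increments the GameInstance counter and picks the level to load from it.
; The first two counts queue the procedural maps, toggle level visibility and request the next load; other counts queue the menu and kill the player.
; A separate Box overlap turns the tile's plane white when the player enters.
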(event OnComponentBeginOverlap(Box)
  (params (OverlappedComponent :type Primitive%20Component%20Object%20Reference) (OtherActor :type Actor%20Object%20Reference) (OtherComp :type Primitive%20Component%20Object%20Reference) (OtherBodyIndex :type Integer) (bFromSweep :type Boolean) (SweepResult :type Hit%20Result%20Structure%20%28by%20ref%29))
  (Utilities|Casting|CastToBP_Player OtherActor)
  (Rendering|Material|SetMaterial (Variables|Default|GetPlane) 0 "/Game/RandomizedDungeons/chars/White.White"))

(event OnComponentBeginOverlap(Restart)
  (params (OverlappedComponent :type Primitive%20Component%20Object%20Reference) (OtherActor :type Actor%20Object%20Reference) (OtherComp :type Primitive%20Component%20Object%20Reference) (OtherBodyIndex :type Integer) (bFromSweep :type Boolean) (SweepResult :type Hit%20Result%20Structure%20%28by%20ref%29))
  (bind _asbp_player (Utilities|Casting|CastToBP_Player OtherActor))
  (bind _asgi_base (Utilities|Casting|CastToGI_Base (Game|GetGameInstance)))
  (Class|BILevels|TileCall(Message) (Class|GameplayStatics|GetStreamingLevel (Variables|/Game/DD/Core/Player/GI_Base.GI_Base_C|GetCurrentLvl _asgi_base)))
  (bind _result (Math|Integer|IncrementInt (Variables|/Game/DD/Core/Player/GI_Base.GI_Base_C|GetCounter _asgi_base))
    (:%20%20
      (switch int _result
        (:Default
          (Variables|/Game/DD/Core/Player/GI_Base.GI_Base_C|SetLvlToLoad _asgi_base "Menu" :!label _label)
          (Default|DIE _asbp_player))
        (:1
          (Variables|/Game/DD/Core/Player/GI_Base.GI_Base_C|SetLvlToLoad _asgi_base "ProcMap1")
          (Variables|/Script/Engine.LevelStreaming|SetbShouldBeVisible (Class|GameplayStatics|GetStreamingLevel (Variables|/Game/DD/Core/Player/GI_Base.GI_Base_C|GetCurrentLvl _asgi_base)) true)
          (Class|BILevels|LoadNextStreamingLevel(Message) (Class|GameplayStatics|GetStreamingLevel (Variables|/Game/DD/Core/Player/GI_Base.GI_Base_C|GetCurrentLvl _asgi_base))))
        (:2
          (Variables|/Game/DD/Core/Player/GI_Base.GI_Base_C|SetLvlToLoad _asgi_base "ProcMap2")
          (Variables|/Script/Engine.LevelStreaming|SetbShouldBeVisible (Class|GameplayStatics|GetStreamingLevel (Variables|/Game/DD/Core/Player/GI_Base.GI_Base_C|GetCurrentLvl _asgi_base)) false)
          (Class|BILevels|LoadNextStreamingLevel(Message) (Class|GameplayStatics|GetStreamingLevel (Variables|/Game/DD/Core/Player/GI_Base.GI_Base_C|GetCurrentLvl _asgi_base))))
        (:3
          (goto _label))))))

(event EventBeginPlay)

(event Collision|EventActorBeginOverlap
  (params (OtherActor :type Actor%20Object%20Reference)))

(event EventTick
  (params (DeltaSeconds :type Float%20%28single-precision%29)))

(fn ConstructionScript)
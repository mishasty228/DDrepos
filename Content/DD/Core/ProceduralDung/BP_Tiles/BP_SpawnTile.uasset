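; BP_SpawnTile is the procedural dungeon tile that places the player and a starting weapon when play begins.
; On BeginPlay it stores its Scene transform as BP_Player's InitLocation, calls GoToSpawn, moves the player's capsule there and sets the GetLocation flag.
; It then spawns a SmallSword at the Scene1 marker.
; A two-second delay before the teleport is left disconnected and never runs.
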(event EventBeginPlay
  (bind _asbp_player (Utilities|Casting|CastToBP_Player (Game|GetPlayerCharacter 0)))
  (bind _output_get (Variables|/Game/DD/Core/Player/BP_Player.BP_Player_C|SetInitLocation _asbp_player (Transformation|GetWorldTransform (Variables|Default|GetScene))))
  (Default|GotoSpawn _asbp_player)
  (Transformation|SetWorldTransform (Variables|/Script/Engine.Character|GetCapsuleComponent (Game|GetPlayerCharacter 0)) _output_get false false)
  (Variables|/Game/DD/Core/Player/BP_Player.BP_Player_C|SetGetLocation _asbp_player true)
  (Game|SpawnActorfromClass "/Game/DD/Core/Inventory/Weapons/SmallSword.SmallSword_C" (Transformation|GetWorldTransform (Variables|Default|GetScene1)) "AdjustIfPossibleButAlwaysSpawn" 0 0))

(event Collision|EventActorBeginOverlap
  (params (OtherActor :type Actor%20Object%20Reference)))

(event EventTick
  (params (DeltaSeconds :type Float%20%28single-precision%29)))

(fn ConstructionScript)
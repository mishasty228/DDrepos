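; GM_Base is a base game mode that, as wired, only caches the game instance, cast to GI_Base, on BeginPlay.
; Unconnected load logic would disable BP_Player input, check for the "Save" slot, then load through GI_Base and re-enable input only if that save exists.
; A separate unconnected call to the game instance's SaveGame also never runs.
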(event EventBeginPlay
  (bind _asgi_base (Utilities|Casting|CastToGI_Base (Game|GetGameInstance)))
  (Variables|Default|SetGI _asgi_base))

(event EventTick
  (params (DeltaSeconds :type Float%20%28single-precision%29)))

(fn ConstructionScript)